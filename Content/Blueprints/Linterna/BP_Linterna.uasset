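; BP_Linterna is a grabbable VR flashlight that switches its spotlight on only while held, with sounds for switch, grab and drop.
; Grab and drop both call LinternaRunServer, then LinternaMulticast, starting a looping timer, so dropping turns off the light but restarts the just-cleared timer.
; The timer writes spotlight position, direction, flashlight state and BP_btonLuz's state into the LinternaParametros Material Parameter Collection for materials to read.
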(event OnGrabbed(GrabComponent)
  (params (Motion%20Controller :type Motion%20Controller%20Component%20Object%20Reference))
  (Variables|Default|SetLinternaCogida true)
  (Audio|PlaySoundatLocation "/Engine/VREditor/Sounds/VR_grab.VR_grab" (Transformation|GetActorLocation) "0, 0, 0" 0.5 1.0 0.0 0 0 0 0)
  (CallFunction|LinternaRunServer))

(event OnDropped(GrabComponent)
  (Audio|PlaySoundatLocation "/Engine/VREditor/Sounds/UI/Drop_Item_From_ContentBrowser.Drop_Item_From_ContentBrowser" (Transformation|GetActorLocation) "0, 0, 0" 0.3 1.0 0.0 0 0 0 0)
  (Variables|Default|SetLinternaCogida false)
  (Utilities|Time|ClearTimerbyFunctionName 0 "ComprobacionPosicionLinterna")
  (CallFunction|Apagar)
  (CallFunction|LinternaRunServer))

(event Custom|Apagar
  (Audio|PlaySoundatLocation "/Engine/VREditor/Sounds/UI/Flashlight_Switch.Flashlight_Switch" (Transformation|GetActorLocation) "0, 0, 0" 0.5 1.0 0.0 0 0 0 0)
  (Rendering|SetVisibility (Variables|Default|GetSpotLight) false false)
  (Variables|Default|SetLinternaLuz false))

(event Custom|Encender
  (bind _spotlight (Variables|Default|GetSpotLight))
  (Audio|PlaySoundatLocation "/Engine/VREditor/Sounds/UI/Flashlight_Switch.Flashlight_Switch" (Transformation|GetActorLocation) "0, 0, 0" 1.0 1.0 0.0 0 0 0 0)
  (if (Variables|Default|GetLinternaCogida)
    (Rendering|SetVisibility _spotlight true false)
    (Variables|Default|SetLinternaLuz true)
    (else
      (Rendering|SetVisibility _spotlight false false)
      (Variables|Default|SetLinternaLuz false))))

(event Custom|LinternaRunServer
  (CallFunction|LinternaMulticast))

(event Custom|LinternaMulticast
  (Utilities|Time|SetTimerbyFunctionName 0 "ComprobacionPosicionLinterna" 0.01 true))

(fn ConstructionScript)

(fn ComprobacionPosicionLinterna
  (bind _spotlight (Variables|Default|GetSpotLight))
  (bind _returnvalue (Actor|GetActorOfClass "/Game/Blueprints/Interruptor/BP_btonLuz/BP_btonLuz.BP_btonLuz_C"))
  (if (Variables|/Game/Blueprints/Interruptor/BP_btonLuz/BP_btonLuz.BP_btonLuz_C|GetEncendido _returnvalue)
    (Rendering|Material|SetVectorParameterValue "/Game/VRTemplate/Blueprints/LinternaParametros.LinternaParametros" "Luz" (Utilities|Struct|MakeLinearColor 1.0 0.0 0.0 0.0) :!class /Script/Engine.KismetMaterialLibrary)
    (else
      (Rendering|Material|SetVectorParameterValue "/Game/VRTemplate/Blueprints/LinternaParametros.LinternaParametros" "Luz" (Utilities|Struct|MakeLinearColor 0.0 0.0 0.0 0.0) :!class /Script/Engine.KismetMaterialLibrary)))
  (Rendering|Material|SetVectorParameterValue "/Game/VRTemplate/Blueprints/LinternaParametros.LinternaParametros" "PosicionLinterna" (Math|Conversions|ToLinearColor(Vector) (Transformation|GetWorldLocation _spotlight)) :!class /Script/Engine.KismetMaterialLibrary)
  (Rendering|Material|SetVectorParameterValue "/Game/VRTemplate/Blueprints/LinternaParametros.LinternaParametros" "FordwardVector" (Math|Conversions|ToLinearColor(Vector) (Math|Vector|GetForwardVector _spotlight)) :!class /Script/Engine.KismetMaterialLibrary)
  (if (Variables|Default|GetLinternaLuz)
    (Rendering|Material|SetVectorParameterValue "/Game/VRTemplate/Blueprints/LinternaParametros.LinternaParametros" "Linterna" (Utilities|Struct|MakeLinearColor 1.0 0.0 0.0 1.0) :!class /Script/Engine.KismetMaterialLibrary)
    (else
      (Rendering|Material|SetVectorParameterValue "/Game/VRTemplate/Blueprints/LinternaParametros.LinternaParametros" "Linterna" (Utilities|Struct|MakeLinearColor 0.0 0.0 0.0 1.0) :!class /Script/Engine.KismetMaterialLibrary))))